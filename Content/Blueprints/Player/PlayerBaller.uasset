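; PlayerBaller is a player Blueprint that turns axis input into movement and look control.
; Move axes add movement input along the forward and right vectors of GetZControlRotation, keeping movement relative to control rotation.
; Separate look and mouse axes pass raw values to controller pitch and yaw.
; The mouse sensitivity scaling and speed-setting logic shown here are unconnected.
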(event Input|AxisEvents|InputAxisMoveForward/Backwards
  (params (AxisValue :type Float%20%28single-precision%29))
  ;[0.1042 0.1042 0.1042] Movement
  (Pawn|Input|AddMovementInput (Math|Vector|GetForwardVector (|GetZControlRotation)) AxisValue false))

(event Input|AxisEvents|InputAxisMoveRight/Left
  (params (AxisValue :type Float%20%28single-precision%29))
  ;[0.1042 0.1042 0.1042] Movement
  (Pawn|Input|AddMovementInput (Math|Vector|GetRightVector (|GetZControlRotation)) AxisValue false))

(event Input|AxisEvents|InputAxisMouseTurn
  (params (AxisValue :type Float%20%28single-precision%29))
  (Pawn|Input|AddControllerYawInput AxisValue))

(event Input|AxisEvents|InputAxisMouseUp
  (params (AxisValue :type Float%20%28single-precision%29))
  (Pawn|Input|AddControllerPitchInput AxisValue))

(event Input|AxisEvents|InputAxisLookUp
  (params (AxisValue :type Float%20%28single-precision%29))
  (Pawn|Input|AddControllerPitchInput AxisValue))

(event Input|AxisEvents|InputAxistURN
  (params (AxisValue :type Float%20%28single-precision%29))
  (Pawn|Input|AddControllerYawInput AxisValue))

(fn ConstructionScript
  (|CallParentFunction))