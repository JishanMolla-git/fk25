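; Pack manager actor that draws a random player card from a pack data asset, weighted by rarity.
; BeginPlay sums every card's RarityWeight into TotalWeight and starts a looping timer, whose bound event is not named.
; OpenPack rolls a truncated random value up to that total, walks the cards accumulating weight, and prints the name of the first to reach it.
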(event Custom|Open%20Pack
  (Variables|Default|SetRandom%20Value (Math|Float|Truncate (Math|Random|RandomFloatinRange 0.0 (Math|Conversions|ToFloat(Integer) (Variables|Default|GetTotal%20Weight)))))
  (Variables|Default|SetAccmulated%20Weight 0)
  (bind _packdataasset (Variables|Default|GetPackDataAsset)
    (:then
      (bind _array_element (Utilities|Array|ForEachLoopwithBreak (Variables|/Game/Blueprints/PACKS/PDA_CardDefinition.PDA_CardDefinition_C|GetPlayer%20Cards _packdataasset) :!label _label)
        (:LoopBody
          (bind _output_get (Variables|Default|SetAccmulated%20Weight (+ (.RarityWeight (Utilities|Struct|BreakST_PlayerCardData _array_element)) (Variables|Default|GetAccmulated%20Weight))))
          (if (>= _output_get (Variables|Default|GetRandom%20Value))
            (Development|PrintText (.Name (Utilities|Struct|BreakST_PlayerCardData _array_element)))
            (goto _label Break)))))
    (:else)))

(event EventBeginPlay
  (Utilities|FlowControl|Sequence
    (:then_0
      (Utilities|Time|SetTimerbyEvent (EventDispatchers|CreateEvent :!event Custom|Open%20Pack) 2.0 true))
    (:then_1
      (CallFunction|CalculateTotalWeight))))

(fn ConstructionScript)

(fn CalculateTotalWeight
  (bind _packdataasset (Variables|Default|GetPackDataAsset)
    (:then
      (for _array_element (Variables|/Game/Blueprints/PACKS/PDA_CardDefinition.PDA_CardDefinition_C|GetPlayer%20Cards _packdataasset)
        (Variables|Default|SetTotal%20Weight (+ (.RarityWeight (Utilities|Struct|BreakST_PlayerCardData _array_element)) (Variables|Default|GetTotal%20Weight)))))
    (:else)))